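; Jumper enemy Blueprint with continuously spinning blades and a body that can hop up and down.
; Tick yaws the Blades component at SpinSpeed scaled by delta time.
; BeginPlay caches the Body's resting relative Z, and StartJump plays a timeline that offsets the Body's height from it.
; EndJump reverses the same timeline to bring the Body back down.
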(event `self.ReceiveBeginPlay`
  (bind (_relativelocation_x _relativelocation_y _relativelocation_z) (`KismetMathLibrary.BreakVector` (`SceneComponent.RelativeLocation` (`self.Body`))))
  (set `self.NormalZ` _relativelocation_z))

(event `self.ReceiveTick`
  (params (DeltaSeconds :type "Float (single-precision)"))
  (`SceneComponent.K2_AddRelativeRotation` (`self.Blades`) (`KismetMathLibrary.MakeRotator` 0.0 0.0 (* DeltaSeconds (`self.SpinSpeed`))) false false))

(event `StartJump`
  (bind (_direction _height) (`Timeline|JumpTimeline` :!label _label)
    (:`Update`
      (`SceneComponent.K2_SetRelativeLocation` (`self.Body`) (`KismetMathLibrary.MakeVector` 0.0 0.0 (+ _height (`self.NormalZ`))) false false))))

(event `EndJump`
  (goto _label :!via `Reverse`))

(fn `UserConstructionScript`)